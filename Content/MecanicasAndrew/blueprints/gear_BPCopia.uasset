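; VR gear Blueprint whose Gear component turns on yaw only to face the player pawn, apparently a work-in-progress grab mechanic.
; Tick applies the look-at rotation unconditionally, then repeats it when Follow is set, so the gear tracks the pawn regardless of grabbing.
; A motion controller overlapping Box stores the hand and permanently sets Canfollow, which GrabRight presses copy into Follow.
; The stored hand is never used.
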(event `self.ReceiveTick`
  (params (DeltaSeconds :type "Float (single-precision)"))
  (bind _gear (`self.gear`))
  (bind (_returnvalue_roll _returnvalue_pitch _returnvalue_yaw) (`KismetMathLibrary.BreakRotator` (`KismetMathLibrary.FindLookAtRotation` (`SceneComponent.K2_GetComponentLocation` _gear) (`self.K2_GetActorLocation` (`self.lookAtPos`)))))
  (bind _returnvalue (`KismetMathLibrary.MakeRotator` 0.0 0.0 _returnvalue_yaw))
  (`|ExecutionSequence`
    (:`then_0`
      (set `self.lookAtPos` (`GameplayStatics.GetPlayerPawn` 0))
      (`SceneComponent.K2_SetWorldRotation` _gear _returnvalue false false :!label _label)
      (set `self.rotation` _returnvalue))
    (:`then_1`
      (if (`self.follow`)
        (goto _label)))))

(event `self.Box.OnComponentBeginOverlap`
  (params (OverlappedComponent :type "PrimitiveComponent Object Reference") (OtherActor :type "Actor Object Reference") (OtherComp :type "PrimitiveComponent Object Reference") (OtherBodyIndex :type Integer) (bFromSweep :type Boolean) (SweepResult :type "HitResult Structure (by ref)"))
  (bind _asmotion_controller_component (cast `MotionControllerComponent` OtherComp))
  (bind _asbp_motion_controller (cast `/Game/VirtualRealityBP/Blueprints/BP_MotionController` (`ActorComponent.GetOwner` _asmotion_controller_component)))
  (set `self.Mano` _asbp_motion_controller)
  (set `self.Canfollow` true)
  (`KismetSystemLibrary.PrintString` "entro"))

(event `InputAction|GrabRight`
  (params (Key :type "Key Structure"))
  (:`Pressed`
    (if (`self.Canfollow`)
      (set `self.follow` true)
      (else
        (set `self.follow` false)))))

(fn `UserConstructionScript`)