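; Bulb slot actor that detects a bulb_BP entering its Box1 trigger and has it placed in the slot.
; When the slot is empty, an overlapping bulb receives PutInplace with the box's world rotation, and the TieneEngrane and IsOverlaping flags are set.
; Any bulb_BP leaving the box clears both flags, allowing the slot to accept a bulb again.
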(event `self.Box1.OnComponentBeginOverlap`
  (params (OverlappedComponent :type "PrimitiveComponent Object Reference") (OtherActor :type "Actor Object Reference") (OtherComp :type "PrimitiveComponent Object Reference") (OtherBodyIndex :type Integer) (bFromSweep :type Boolean) (SweepResult :type "HitResult Structure (by ref)"))
  (if (not (`self.TieneEngrane`))
    (bind _asbulb_bp (cast `/Game/MecanicasAndrew/blueprints/bulb_BP` OtherActor))
    (`/Game/MecanicasAndrew/blueprints/bulb_BP.Put inplace` _asbulb_bp (`SceneComponent.K2_GetComponentRotation` (`self.Box1`)))
    (set `self.TieneEngrane` true)
    (set `self.isOverlaping` true)))

(event `self.Box1.OnComponentEndOverlap`
  (params (OverlappedComponent :type "PrimitiveComponent Object Reference") (OtherActor :type "Actor Object Reference") (OtherComp :type "PrimitiveComponent Object Reference") (OtherBodyIndex :type Integer))
  (cast `/Game/MecanicasAndrew/blueprints/bulb_BP` OtherActor)
  (set `self.TieneEngrane` false)
  (set `self.isOverlaping` false))

(fn `UserConstructionScript`)