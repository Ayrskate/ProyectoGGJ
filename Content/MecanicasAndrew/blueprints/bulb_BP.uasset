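; A grabbable light bulb actor that can be carried by hand, set in place and used to switch a point light on and off.
; While FollowingHand is set, Tick lerps its location and rotation toward the parent's hand transform.
; Drop and PutInplace stop following and disable physics simulation, with PutInplace also orienting the mesh from a given direction.
; Overlap events set the light's intensity according to the ActiveBulb's overlap flag.
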(event `self.ReceiveTick`
  (params (DeltaSeconds :type "Float (single-precision)"))
  (`|ExecutionSequence`
    (:`then_0`
      (if (`self.FollowingHand`)
        (`self.K2_SetActorLocation` (`KismetMathLibrary.VLerp` (`self.K2_GetActorLocation`) (`/Game/VirtualRealityBP/Blueprints/BP_MotionController.HandPosition` (`self.Parent`)) (* (`self.velSmooth`) DeltaSeconds)))
        (`self.K2_SetActorRotation` (`KismetMathLibrary.RLerp` (`self.K2_GetActorRotation`) (`/Game/VirtualRealityBP/Blueprints/BP_MotionController.HandRotation` (`self.Parent`))))))))

(event `Event PickUp`
  (if (`self.Attached`)
    _))

(event `Event Drop`
  (bind _staticmesh (`self.StaticMesh`))
  (set `self.FollowingHand` false)
  (`PrimitiveComponent.SetEnableGravity` (`self.StaticMesh`) false)
  (`PrimitiveComponent.SetLinearDamping` _staticmesh 0.0)
  (`PrimitiveComponent.SetAngularDamping` _staticmesh 0.0)
  (`PrimitiveComponent.SetSimulatePhysics` (`self.StaticMesh`) false))

(event `self.ReceiveActorBeginOverlap`
  (params (OtherActor :type "Actor Object Reference"))
  (if (`/Game/MecanicasAndrew/blueprints/bulb_space_BP.isOverlaping` (`self.activeBulb`))
    (`LightComponent.SetIntensity` (`PointLight.PointLightComponent` (`self.light`)) 60.0)))

(event `self.ReceiveActorEndOverlap`
  (params (OtherActor :type "Actor Object Reference"))
  (if (not (`/Game/MecanicasAndrew/blueprints/bulb_space_BP.isOverlaping` (`self.activeBulb`)))
    (`LightComponent.SetIntensity` (`PointLight.PointLightComponent` (`self.light`)) 0.0)))

(fn `Put inplace`
  (params (ForwardDirection :type "Rotator Structure"))
  (bind _parent (`self.Parent`))
  (bind _staticmesh (`self.StaticMesh`))
  (set `self.FollowingHand` false)
  (`/Engine/EditorBlueprintResources/StandardMacros.IsValid` _parent
    (:`Is Valid`
      (set `self.Parent` _parent))
    (:`Is Not Valid`
      _))
  (`SceneComponent.K2_SetWorldRotation` _staticmesh (`KismetMathLibrary.ComposeRotators` ForwardDirection (struct :`Pitch` 90.0)) false false)
  (`PrimitiveComponent.SetSimulatePhysics` _staticmesh false))

(fn `UserConstructionScript`)