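; Checker Blueprint that polls an array of objects every Tick for their IsOverlaping flag, apparently to detect when a set of them is lit.
; For each overlapping element it sets Cont from the incremented loop index, so Cont reflects array position instead of a tally.
; When Cont reaches seven or more it calls LoopBreaker, which only prints a "prendidos" debug message and does not exit the loop.
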(event `self.ReceiveTick`
  (params (DeltaSeconds :type "Float (single-precision)"))
  (for (_array_element _array_index) (`self.01`)
    (if (`/Game/MecanicasAndrew/blueprints/bulb_space_BP.isOverlaping` _array_element)
      (bind _result (`/Engine/EditorBlueprintResources/StandardMacros.IncrementInt` _array_index)
        (:`  `
          (bind _output_get (set `self.cont` _result))
          (if (>= _output_get 7)
            (`self.loopBreaker`)))))))

(fn `loopBreaker`
  (`KismetSystemLibrary.PrintString` "prendidos!!!!!"))

(fn `UserConstructionScript`)