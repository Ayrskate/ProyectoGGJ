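; boolChecker_BP is a checker for a gear-completion mechanic, judging by its folder, that watches the Overlaping flag on an array of elements.
; Every Tick it loops the array and, for each overlapping element, sets Cont from the incremented loop index rather than a running tally.
; When Cont reaches three or more, it calls LoopBreaker, which only prints an all-lit debug message and does not stop the loop.
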(event `self.ReceiveTick`
  (params (DeltaSeconds :type "Float (single-precision)"))
  (for (_array_element _array_index) (`self.array`)
    (if (`/Game/MecanicasPunky/EngranesCompletar/bulb_place.overlaping` _array_element)
      (bind _result (`/Engine/EditorBlueprintResources/StandardMacros.IncrementInt` _array_index)
        (:`  `
          (bind _output_get (set `self.cont` _result))
          (if (>= _output_get 3)
            (`self.loopBreaker`)))))))

(fn `loopBreaker`
  (`KismetSystemLibrary.PrintString` "prendidos todos<!!!"))

(fn `UserConstructionScript`)